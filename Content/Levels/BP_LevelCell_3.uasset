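; BP_LevelCell_3 is a level cell actor with doors on its left, right, top and bottom sides.
; On BeginPlay it casts each door component's child actor to Door and stores the references in per-side variables.
; The casts run in sequence, so a failed cast leaves the remaining doors unassigned.
; It has no other active logic.
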(event EventBeginPlay
  (bind _asdoor (Utilities|Casting|CastToDoor (Variables|/Script/Engine.ChildActorComponent|GetChildActor (Variables|Default|GetDoor_Left_C))))
  (Variables|Default|Set_doorLeft _asdoor)
  (bind _asdoor_2 (Utilities|Casting|CastToDoor (Variables|/Script/Engine.ChildActorComponent|GetChildActor (Variables|Default|GetDoor_Right_C))))
  (Variables|Default|Set_doorRight _asdoor_2)
  (bind _asdoor_3 (Utilities|Casting|CastToDoor (Variables|/Script/Engine.ChildActorComponent|GetChildActor (Variables|Default|GetDoor_Top_C))))
  (Variables|Default|Set_doorTop _asdoor_3)
  (bind _asdoor_4 (Utilities|Casting|CastToDoor (Variables|/Script/Engine.ChildActorComponent|GetChildActor (Variables|Default|GetDoor_Bottom_C))))
  (Variables|Default|Set_doorBottom _asdoor_4))

(event Collision|EventActorBeginOverlap
  (params (OtherActor :type Actor%20Object%20Reference)))

(event EventTick
  (params (DeltaSeconds :type Float%20%28single-precision%29)))

(fn ConstructionScript)